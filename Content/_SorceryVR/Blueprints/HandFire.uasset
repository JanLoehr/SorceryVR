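; HandFire is a VR fire object that attaches to the grabbing hand and can be shot on release.
; While held, Tick compares the X component of the hand's MagicAnchor forward vector with the camera-to-hand direction, turning the light red and arming the shot within ShootTolerance.
; Pickup disables mesh physics; Drop detaches and, if armed, applies a forward velocity impulse with controller rumble, without explicitly re-enabling physics.
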(event `self.ReceiveTick`
  (params (DeltaSeconds :type "Float (single-precision)"))
  (bind _holdinghand (`self.HoldingHand`))
  (bind _light (`self.Light`))
  (bind _shoottolerance (`self.ShootTolerance`))
  ;[1 1 1] Check if fire was shot, and shoot it
  (if (`self.IsGrabbed`)
    (bind _asbp_motion_controller (cast `/Game/VirtualRealityBP/Blueprints/BP_MotionController` (`ActorComponent.GetOwner` _holdinghand)))
    (if (`KismetMathLibrary.InRange_FloatFloat` (.x (- (`SceneComponent.GetForwardVector` (`/Game/VirtualRealityBP/Blueprints/BP_MotionController.MagicAnchor` _asbp_motion_controller)) (`KismetMathLibrary.GetDirectionUnitVector` (`PlayerCameraManager.GetCameraLocation` (`GameplayStatics.GetPlayerCameraManager` 0)) (`SceneComponent.K2_GetComponentLocation` _holdinghand)))) (- 0.0 _shoottolerance) (+ 0.0 _shoottolerance))
      (`LightComponent.SetLightColor` _light (struct :`R` 1.0 :`B` 0.046985 :`A` 1.0) true)
      (set `self.ShouldShoot` true)
      (else
        (`LightComponent.SetLightColor` _light (struct :`R` 1.0 :`G` 1.0 :`B` 1.0 :`A` 1.0) true)
        (set `self.ShouldShoot` false)))))

(event `/Game/VirtualRealityBP/Blueprints/PickupActorInterface.Drop`
  (params (DroppingHand :type "/Game/VirtualRealityBP/Blueprints/BP_MotionController Object Reference"))
  ;[1 1 1] Drop
  (set `self.IsGrabbed` false)
  (`self.K2_DetachFromActor` "KeepRelative")
  ;[1 1 1] Add Force if shot
  (if (`self.ShouldShoot`)
    (`PrimitiveComponent.AddImpulse` (`self.StaticMesh`) (* (`SceneComponent.GetForwardVector` (`/Game/VirtualRealityBP/Blueprints/BP_MotionController.MagicAnchor` DroppingHand)) 1000.0) "None" true)
    (`/Game/VirtualRealityBP/Blueprints/BP_MotionController.RumbleController` DroppingHand 0.5)))

(event `/Game/VirtualRealityBP/Blueprints/PickupActorInterface.Pickup`
  (params (AttachTo :type "SceneComponent Object Reference"))
  ;[1 1 1] Pickup
  (bind _output_get (set `self.HoldingHand` AttachTo))
  (set `self.IsGrabbed` true)
  (`PrimitiveComponent.SetSimulatePhysics` (`self.StaticMesh`) false)
  (`self.K2_AttachToComponent` _output_get "None" "KeepWorld" "KeepWorld" "KeepWorld" false))

(fn `UserConstructionScript`)